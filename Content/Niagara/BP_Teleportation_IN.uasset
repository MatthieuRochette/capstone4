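; BP_Teleportation_IN plays the teleport-in arrival of the Tractopelle actor when play begins.
; BeginPlay hides the Tractopelle, starts a Level Sequence, audio and a Niagara effect, then reveals it after a short delay.
; When the sequence finishes on EndLevel, it shows the WBP_Win widget with the mouse cursor and UI-only input.
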(event `self.ReceiveBeginPlay`
  ;[1 1 1] Teleportation In Process
  (`self.SetActorHiddenInGame` (`self.Tractopelle`) true)
  (bind (_outactor _returnvalue) (`LevelSequencePlayer.CreateLevelSequencePlayer` (`self.CurrentSequence`)))
  (`MovieSceneSequencePlayer.Play` _returnvalue)
  (add `MovieSceneSequencePlayer.OnFinished` _returnvalue (delegate `OnFinished_Event_0`))
  (`AudioComponent.Play` (`self.Audio`) 2.0)
  (`ActorComponent.Activate` (`NiagaraActor.NiagaraComponent` (`self.NS_Teleportation_IN`)) false)
  (`KismetSystemLibrary.Delay` 1.5)
  (`self.SetActorHiddenInGame` (`self.Tractopelle`) false))

(event `OnFinished_Event_0`
  (bind _returnvalue (`GameplayStatics.GetPlayerController` 0))
  ;[1 1 1] Detect End Level
  (bind _returnvalue_2 (`GameplayStatics.GetCurrentLevelName` true))
  (if (`KismetStringLibrary.EqualEqual_StrStr` _returnvalue_2 "EndLevel")
    (bind _returnvalue_3 (`|CreateWidget` "/Game/UI/WBP_Win.WBP_Win_C" _returnvalue))
    (`UserWidget.AddToViewport` _returnvalue_3 0)
    (set `PlayerController.bShowMouseCursor` true _returnvalue)
    (`WidgetBlueprintLibrary.SetInputMode_UIOnlyEx` _returnvalue _returnvalue_3)))

(fn `UserConstructionScript`)