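; Teleportation trigger actor that sends the game to the "Test" level when any actor overlaps it.
; On overlap it adds and activates a Niagara component on the Tractopelle actor and plays Audio1.
; After timed delays it hides Tractopelle, then opens the level by name.
; The overlap has no actor filter or re-entry guard, and the NSTeleportation component reference is left unused.
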(event `self.ReceiveActorBeginOverlap`
  (params (OtherActor :type "Actor Object Reference"))
  (bind _tractopelle (`self.Tractopelle`))
  (bind _returnvalue (`AddComponent|NODE_AddNiagaraComponent-1` :`self` _tractopelle))
  (`ActorComponent.Activate` _returnvalue false)
  (`AudioComponent.Play` (`self.Audio1`) -0.3)
  (`KismetSystemLibrary.Delay` 2.0)
  (`self.SetActorHiddenInGame` _tractopelle true)
  (`KismetSystemLibrary.Delay` 0.5)
  (`GameplayStatics.OpenLevel` "Test"))

(fn `UserConstructionScript`)