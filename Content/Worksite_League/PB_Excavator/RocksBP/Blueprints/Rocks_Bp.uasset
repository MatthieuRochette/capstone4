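; Rock pile actor whose rocks break loose into physics bodies when hit by BP_Excavator.
; The construction script fills a HISM with a 3D grid of randomly rotated rocks.
; On hit, a sphere trace recovers the instance index, then that instance is swapped for a simulating static mesh with debris FX and sound.
; When simulating rocks exceed the limit, all of them are destroyed at once.
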(event `self.RockHISMC.OnComponentHit`
  (params (HitComponent :type "PrimitiveComponent Object Reference") (OtherActor :type "Actor Object Reference") (OtherComp :type "PrimitiveComponent Object Reference") (NormalImpulse :type "Vector Structure") (Hit :type "HitResult Structure (by ref)"))
  (bind (_bblockinghit _binitialoverlap _time _distance _location) (`GameplayStatics.BreakHitResult` Hit))
  (bind _arrayofmeshc (`self.ArrayOfMeshC`))
  ;[1 1 1] Spawn Physic simulating rocks
  (bind _asbp_excavator (cast `/Game/Worksite_League/PB_Excavator/BP_Excavator/Blueprints/BP_Excavator` OtherActor))
  (bind (_outhit _returnvalue) (`KismetSystemLibrary.SphereTraceSingle` _location (+ _location (0.1 0.1 0.1)) 50.0 "TraceTypeQuery1" false (`|MakeArray` _asbp_excavator :!type "Actor Object Reference") "None" false))
  (if _returnvalue
    (bind _ashierarchical_instanced_static_mesh_component (cast `HierarchicalInstancedStaticMeshComponent` HitComponent))
    (bind (_bblockinghit_2 _binitialoverlap_2 _time_2 _distance_2 _location_2 _impactpoint _normal _impactnormal _physmat _hitactor _hitcomponent _hitbonename _hititem) (`GameplayStatics.BreakHitResult` _outhit))
    (bind (_outinstancetransform _returnvalue_2) (`InstancedStaticMeshComponent.GetInstanceTransform` _ashierarchical_instanced_static_mesh_component _hititem true))
    (if _returnvalue_2
      (`self.F_CollapseFX` _impactpoint _impactnormal)
      ;;[1 1 1] Store Transforms
      (set `self.TemporaryIT` _outinstancetransform)
      ;;[1 1 1] Remove instance of the HISMC
      (bind _returnvalue_3 (`InstancedStaticMeshComponent.RemoveInstance` _ashierarchical_instanced_static_mesh_component _hititem))
      (if _returnvalue_3
        ;;[1 1 1] Create a new static mesh component
        (bind _returnvalue_4 (`AddComponent|NODE_AddStaticMeshComponent-0`))
        (`StaticMeshComponent.SetStaticMesh` _returnvalue_4 (`StaticMeshComponent.StaticMesh` (`self.RockHISMC`)))
        ;;[1 1 1] Set world transforms to the instance transforms
        (`SceneComponent.K2_SetWorldTransform` _returnvalue_4 (`self.TemporaryIT`) false true)
        ;;[1 1 1] Mass of the rocks
        (`PrimitiveComponent.SetMassOverrideInKg` _returnvalue_4 "None" (`self.OneRockMassKG`) true)
        (`PrimitiveComponent.SetSimulatePhysics` _returnvalue_4 true)
        ;;[1 1 1] Store into an array
        (`KismetArrayLibrary.Array_AddUnique` (`self.ArrayOfMeshC`) _returnvalue_4)
        (if (> (`KismetArrayLibrary.Array_Length` (`self.ArrayOfMeshC`)) (`self.MaxMeshSimulatingPhysics`))
          ;[1 1 1] Destroy the static mesh components
          (for _array_element (`self.ArrayOfMeshC`)
            (`ActorComponent.K2_DestroyComponent` _array_element))
          (`KismetArrayLibrary.Array_Clear` _arrayofmeshc)
          (`KismetArrayLibrary.Array_Resize` _arrayofmeshc))))))

(fn `F_CollapseFX`
  (params (Location :type "Vector Structure") (ImpactNormal :type "Vector Structure"))
  (`GameplayStatics.PlaySoundAtLocation` "/Game/Worksite_League/PB_Excavator/SFX/SC_RockFallingRandom.SC_RockFallingRandom" Location (struct) 1.0 1.0 0.0 null null null)
  (`GameplayStatics.SpawnEmitterAtLocation` "/Game/Worksite_League/PB_Excavator/StarterContent/Particles/P_Debris.P_Debris" Location (`KismetMathLibrary.Conv_VectorToRotator` ImpactNormal)))

(fn `UserConstructionScript`
  (bind _rockscale (`self.RockScale`))
  (bind _returnvalue (* (`self.RockScale`) (`self.RockDistance`)))
  ;[1 1 1] Set the static mesh to the one you want
  (`StaticMeshComponent.SetStaticMesh` (`self.RockHISMC`) (`self.RockStaticMesh`))
  ;[1 1 1] Basic XYZ array of 15x15x15
  (for _index (range (+ (`self.SizeX`) 1))
    (for _index_2 (range (+ (`self.SizeY`) 1))
      (for _index_3 (range (+ (`self.SizeZ`) 1))
        (`InstancedStaticMeshComponent.AddInstance` (`self.RockHISMC`) (`KismetMathLibrary.MakeTransform` (`KismetMathLibrary.MakeVector` (* _index _returnvalue) (* _index_2 _returnvalue) (* _index_3 _returnvalue)) (`KismetMathLibrary.RandomRotator` true) (`KismetMathLibrary.MakeVector` _rockscale _rockscale _rockscale)))))))