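; Interactable world actor that registers itself with BP_Player_Interact while that character is inside its sphere, clearing the reference on exit.
; Each overlap begin or end toggles a floating prompt text, hidden at BeginPlay and rotated on Tick toward the player's follow camera while visible.
; PlayInteractSound and InteractAction events supply the default response: a 2D sound and destroying the actor, respectively.
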(event `self.ReceiveBeginPlay`
  ;[1 1 1] Set Text (content, visibility & position)
  (`TextRenderComponent.K2_SetText` (`self.InteractTextRender`) (`self.InteractText`))
  (bind _output_get (set `self.IsTextInteractionVisible` false))
  (`SceneComponent.SetVisibility` (`self.InteractTextRender`) _output_get true)
  (`SceneComponent.K2_AddWorldOffset` (`self.InteractTextRender`) (`self.InteractTextLocation`) false false))

(event `self.ReceiveTick`
  (params (DeltaSeconds :type "Float (single-precision)"))
  ;[1 1 1] Rotate Text when toggled ON
  (if (`self.IsTextInteractionVisible`)
    (`self.RotateInteractTextTowardsPlayer`)))

(event `PlayInteractSound`
  ;[1 1 1] Sound to play by default on interaction
  (`GameplayStatics.SpawnSound2D` (`self.InteractSound`) 1.0 1.0 0.0 null))

(event `InteractAction`
  ;[1 1 1] Default Action on interaction
  (`self.K2_DestroyActor`))

(event `self.Sphere.OnComponentBeginOverlap`
  (params (OverlappedComponent :type "PrimitiveComponent Object Reference") (OtherActor :type "Actor Object Reference") (OtherComp :type "PrimitiveComponent Object Reference") (OtherBodyIndex :type Integer) (bFromSweep :type Boolean) (SweepResult :type "HitResult Structure (by ref)"))
  ;[1 1 1] Set object as interactable in character + toggle text
  (bind _asbp_player_interact (cast `/Game/Worksite_League/InteractableActor/BP_Player_Interact` OtherActor))
  (`/Game/Worksite_League/InteractableActor/BP_Player_Interact.SetCurrentInteractableActor` _asbp_player_interact self)
  (`self.ToggleInteractTextRender` :!label _label))

(event `self.Sphere.OnComponentEndOverlap`
  (params (OverlappedComponent :type "PrimitiveComponent Object Reference") (OtherActor :type "Actor Object Reference") (OtherComp :type "PrimitiveComponent Object Reference") (OtherBodyIndex :type Integer))
  ;[1 1 1] Set object as interactable in character + toggle text
  (bind _asbp_player_interact (cast `/Game/Worksite_League/InteractableActor/BP_Player_Interact` OtherActor))
  (`/Game/Worksite_League/InteractableActor/BP_Player_Interact.SetCurrentInteractableActor` _asbp_player_interact null)
  (goto _label))

(fn `RotateInteractTextTowardsPlayer`
  (bind _asthird_person_character (cast `/Game/ThirdPersonBP/Blueprints/ThirdPersonCharacter` (`GameplayStatics.GetPlayerCharacter` 0)))
  (`SceneComponent.K2_SetWorldRotation` (`self.InteractTextRender`) (`KismetMathLibrary.FindLookAtRotation` (`self.K2_GetActorLocation`) (`SceneComponent.K2_GetComponentLocation` (`/Game/ThirdPersonBP/Blueprints/ThirdPersonCharacter.FollowCamera` _asthird_person_character))) false false))

(fn `ToggleInteractTextRender`
  (bind _returnvalue (not (`self.IsTextInteractionVisible`)))
  (`SceneComponent.SetVisibility` (`self.InteractTextRender`) _returnvalue true)
  (set `self.IsTextInteractionVisible` _returnvalue))

(fn `UserConstructionScript`
  (set `self.IsTextInteractionVisible` (`SceneComponent.bVisible` (`self.InteractTextRender`))))