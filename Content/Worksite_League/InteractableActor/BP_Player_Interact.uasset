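; BP_Player_Interact is the on-foot player Blueprint that picks up items and boards excavators in Worksite League.
; It adds a crosshair on BeginPlay and stores interactable and excavator references supplied through setter events.
; Interact on an overlapped item plays PickItem, then after a delay destroys it and calls DropItem on every excavator.
; Without an interactable, it possesses the excavator, shows its driver, removes the HUD and destroys itself.
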(event `self.ReceiveBeginPlay`
  (`self.CreateUI`)
  (`parent.ReceiveBeginPlay`))

(event `SetCurrentExcavatorRef`
  (params (ExcavatorRef :type "/Game/Worksite_League/PB_Excavator/BP_Excavator/Blueprints/BP_Excavator Object Reference"))
  (set `self.ExcavatorRef` ExcavatorRef))

(event `SetCurrentInteractableActor`
  (params (`Actor ref` :type "/Game/Worksite_League/InteractableActor/BP_InteractableActor Object Reference"))
  (set `self.InteractableActorRef` `Actor ref`))

(event `InputAction|Interact`
  (params (Key :type "Key Structure"))
  (bind _interactableactorref (`self.InteractableActorRef`))
  (bind _excavatorref (`self.ExcavatorRef`))
  ;[1 0.7014 0.528] Interactions
  (:`Pressed`
    (`/Engine/EditorBlueprintResources/StandardMacros.IsValid` _interactableactorref
      (:`Is Valid`
        ;;[0.7917 1 0.5833] Actions with interactable object
        (if (`self.IsOverlappingActor` self _interactableactorref)
          (`AudioComponent.Play` (`self.PickItem`) 0.0)
          (`KismetSystemLibrary.Delay` 0.7)
          (`self.K2_DestroyActor` _interactableactorref)
          (bind _outactors (`GameplayStatics.GetAllActorsOfClass` "/Game/Worksite_League/PB_Excavator/BP_Excavator/Blueprints/BP_Excavator.BP_Excavator_C"))
          (for _array_element _outactors
            (`/Game/Worksite_League/PB_Excavator/BP_Excavator/Blueprints/BP_Excavator.Drop Item` _array_element))))
      (:`Is Not Valid`
        ;;[0.604 0.7666 1] Actions with Excavator
        (`/Engine/EditorBlueprintResources/StandardMacros.IsValid` _excavatorref
          (:`Is Valid`
            (`Controller.Possess` (`GameplayStatics.GetPlayerController` 0) _excavatorref)
            (`SceneComponent.SetVisibility` (`/Game/Worksite_League/PB_Excavator/BP_Excavator/Blueprints/BP_Excavator.Driver` _excavatorref) true true)
            (`Widget.RemoveFromParent` (`self.Crosshair`))
            (`Widget.RemoveFromParent` (`self.HealthBar`))
            (`self.K2_DestroyActor`)))))))

(fn `CreateUI`
  (bind _returnvalue (`|CreateWidget` "/Game/Worksite_League/InteractableActor/WBP_Crosshair.WBP_Crosshair_C"))
  (bind _output_get (set `self.Crosshair` _returnvalue))
  (`UserWidget.AddToViewport` _output_get 0))

(fn `UserConstructionScript`
  (`parent.UserConstructionScript`))