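; BP_LargerChaser is an enemy that chases the player and plays random monster sounds at random intervals.
; Perceiving the player or taking damage sets Attack, which drives an AIMoveTo toward the player on Tick while it is alive.
; Hitting the player pauses the chase for DelayBetweenAttacks with a back-off animation.
; Die stops movement, flags death in BP_Chaser_Anim and destroys the actor after timed delays.
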(event `self.ReceiveTick`
  (params (DeltaSeconds :type "Float (single-precision)"))
  (bind _audio (`self.Audio`))
  (`|ExecutionSequence`
    (:`then_0`
      ;[1 1 1] Play monster sound
      (`/Engine/EditorBlueprintResources/StandardMacros.DoOnce` false :!label _label
        (:`Completed`
          (`AudioComponent.SetSound` _audio (`KismetArrayLibrary.Array_Random` (`self.Sounds`)))
          (`AudioComponent.Play` _audio 0.0)
          (`KismetSystemLibrary.Delay` (`KismetMathLibrary.RandomFloatInRange` 2.0 8.0))
          (goto _label :!via `Reset`))))
    (:`then_1`
      ;[1 1 1] AI movement
      (if (`self.Attack`)
        (if (`self.IsAlive`)
          (`|AIMoveTo` self (0.0 0.0 0.0) (`GameplayStatics.GetPlayerCharacter` 0)))))))

(event `self.AIPerception.OnTargetPerceptionUpdated`
  (params (Actor :type "Actor Object Reference") (Stimulus :type "AIStimulus Structure"))
  (cast `/Game/Blueprints/BP_Player` Actor)
  (set `self.Attack` true)
  (bind _asbp_chaser_anim (cast `/Game/CityofBrass_Enemies/Meshes/Enemy/Corpse/BP_Chaser_Anim` (`SkeletalMeshComponent.GetAnimInstance` (`self.Mesh`))))
  (set `/Game/CityofBrass_Enemies/Meshes/Enemy/Corpse/BP_Chaser_Anim.attack` true _asbp_chaser_anim))

(event `self.CapsuleComponent.OnComponentHit`
  (params (HitComponent :type "PrimitiveComponent Object Reference") (OtherActor :type "Actor Object Reference") (OtherComp :type "PrimitiveComponent Object Reference") (NormalImpulse :type "Vector Structure") (Hit :type "HitResult Structure (by ref)"))
  (cast `/Game/Blueprints/BP_Player` OtherActor)
  (bind _asbp_chaser_anim (cast `/Game/CityofBrass_Enemies/Meshes/Enemy/Corpse/BP_Chaser_Anim` (`SkeletalMeshComponent.GetAnimInstance` (`self.Mesh`))))
  (set `self.Attack` false)
  (set `/Game/CityofBrass_Enemies/Meshes/Enemy/Corpse/BP_Chaser_Anim.attack` false _asbp_chaser_anim)
  (set `/Game/CityofBrass_Enemies/Meshes/Enemy/Corpse/BP_Chaser_Anim.back` true _asbp_chaser_anim)
  (`KismetSystemLibrary.Delay` (`self.DelayBetweenAttacks`))
  (set `self.Attack` true)
  (set `/Game/CityofBrass_Enemies/Meshes/Enemy/Corpse/BP_Chaser_Anim.back` false _asbp_chaser_anim)
  (set `/Game/CityofBrass_Enemies/Meshes/Enemy/Corpse/BP_Chaser_Anim.attack` true _asbp_chaser_anim))

(event `self.Die`
  (`NavMovementComponent.StopActiveMovement` (`self.CharacterMovement`))
  (bind _asbp_chaser_anim (cast `/Game/CityofBrass_Enemies/Meshes/Enemy/Corpse/BP_Chaser_Anim` (`SkeletalMeshComponent.GetAnimInstance` (`self.Mesh`))))
  (set `/Game/CityofBrass_Enemies/Meshes/Enemy/Corpse/BP_Chaser_Anim.death` true _asbp_chaser_anim)
  (`KismetSystemLibrary.Delay` 0.2)
  (set `self.IsAlive` false)
  (`KismetSystemLibrary.Delay` 2.6333)
  (`self.K2_DestroyActor`))

(event `self.TakeDamages`
  (bind _asbp_chaser_anim (cast `/Game/CityofBrass_Enemies/Meshes/Enemy/Corpse/BP_Chaser_Anim` (`SkeletalMeshComponent.GetAnimInstance` (`self.Mesh`))))
  (set `/Game/CityofBrass_Enemies/Meshes/Enemy/Corpse/BP_Chaser_Anim.attack` true _asbp_chaser_anim)
  (set `self.Attack` true))

(fn `UserConstructionScript`)