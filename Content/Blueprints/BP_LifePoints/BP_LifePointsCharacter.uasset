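; BP_LifePointsCharacter is a character base with health and death handling for players and monsters, split by an IsMonster flag.
; Capsule hits apply damage: rifle rounds hurt monsters, while monster contact and Grenadier grenades hurt non-monsters, throttled by DoOnce and attack-delay cooldowns.
; Monsters are destroyed at zero health; players spend a GameInstance life to respawn at their start transform, or get the game-over widget.
; A health bar widget updates every Tick, shown only for BP_Player.
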(event `PlayerDeath`
  (bind _returnvalue (`GameplayStatics.GetPlayerController` 0))
  ;[1 1 1] Deaths
  (bind _asfps_game_instance (cast `/Game/Blueprints/FPS_GameInstance` (`GameplayStatics.GetGameInstance`)))
  (bind _result (`/Engine/EditorBlueprintResources/StandardMacros.DecrementInt` (`/Game/Blueprints/FPS_GameInstance.RemainingLives` _asfps_game_instance))
    (:`  `
      (if (>= _result 0)
        (`self.K2_SetActorTransform` (`self.SpawnTransform`) false true)
        (`self.Refill Health`)
        (else
          (set `self.IsAlive` false)
          (set `PlayerController.bShowMouseCursor` true _returnvalue)
          (`WidgetBlueprintLibrary.SetInputMode_UIOnlyEx` _returnvalue null)
          (bind _returnvalue_2 (`|CreateWidget` "/Game/UI/WBP_GameOver.WBP_GameOver_C"))
          (`UserWidget.AddToViewport` _returnvalue_2 0))))))

(event `Die`
  ;[1 1 1] Deaths
  (`NavMovementComponent.StopActiveMovement` (`self.CharacterMovement`))
  (set `self.IsAlive` false)
  (`self.K2_DestroyActor`))

(event `TakeDamages`)

(event `self.CapsuleComponent.OnComponentHit`
  (params (HitComponent :type "PrimitiveComponent Object Reference") (OtherActor :type "Actor Object Reference") (OtherComp :type "PrimitiveComponent Object Reference") (NormalImpulse :type "Vector Structure") (Hit :type "HitResult Structure (by ref)"))
  (bind _returnvalue (`KismetSystemLibrary.GetDisplayName` self))
  (bind _returnvalue_2 (`KismetSystemLibrary.GetDisplayName` self))
  (bind _returnvalue_3 (`KismetSystemLibrary.GetDisplayName` self))
  ;[1 1 1] Hit by bullet/round
  (bind _asbp_assault_rifle_round (cast `/Game/MilitaryWeapSilver/Rounds/BP_AssaultRifleRound` OtherActor)
    (:`then`
      (if (`self.IsMonster`)
        (`self.TakeDamages`)
        (bind _output_get (set `self.HealthPoints` (- (`self.HealthPoints`) 25)))
        (if (<= _output_get 0)
          (`self.Die`)
          (`KismetSystemLibrary.PrintString` (`KismetStringLibrary.Concat_StrStr` _returnvalue_3 ": CHARACTER DIES"))
          (else
            (`KismetSystemLibrary.PrintString` (`KismetStringLibrary.Concat_StrStr` _returnvalue_3 ":" (`KismetStringLibrary.Conv_IntToString` _output_get)))))
        (`self.K2_DestroyActor` _asbp_assault_rifle_round)))
    (:`CastFailed`
      ;[1 1 1] Damages on collision between monster and player
      (bind _asbp_life_points_character (cast `/Game/Blueprints/BP_LifePoints/BP_LifePointsCharacter` OtherActor)
        (:`then`
          (if (`/Game/Blueprints/BP_LifePoints/BP_LifePointsCharacter.IsMonster` _asbp_life_points_character)
            (if (`self.IsMonster`)
              _
              (elif (`/Game/Blueprints/BP_LifePoints/BP_LifePointsCharacter.IsAlive` _asbp_life_points_character)
                (if (`self.IsAlive`)
                  (`/Engine/EditorBlueprintResources/StandardMacros.DoOnce` false :!label _label
                    (:`Completed`
                      (bind _output_get_2 (set `self.HealthPoints` (- (`self.HealthPoints`) (`/Game/Blueprints/BP_LifePoints/BP_LifePointsCharacter.MonsterDamagePoints` _asbp_life_points_character))))
                      (if (<= _output_get_2 0)
                        (`self.PlayerDeath`)
                        (`KismetSystemLibrary.PrintString` (`KismetStringLibrary.Concat_StrStr` _returnvalue_2 ": CHARACTER DIES"))
                        (`KismetSystemLibrary.Delay` (`/Game/Blueprints/BP_LifePoints/BP_LifePointsCharacter.DelayBetweenAttacks` _asbp_life_points_character) :!label _label_2)
                        (goto _label :!via `Reset`)
                        (else
                          (`|ExecutionSequence`
                            (:`then_0`
                              (`GameplayStatics.SpawnEmitterAttached` "/Game/Realistic_Starter_VFX_Pack_Vol2/Particles/Blood/P_Blood_Splat_Cone.P_Blood_Splat_Cone" (`self.Mesh`) "None" (0.0 0.0 0.0) (struct) (2.0 2.0 2.0))
                              (`KismetSystemLibrary.PrintString` (`KismetStringLibrary.Concat_StrStr` _returnvalue_2 ":" (`KismetStringLibrary.Conv_IntToString` _output_get_2))))
                            (:`then_1`
                              (goto _label_2))))))))))))
        (:`CastFailed`
          ;[1 1 1] Damage by grenade
          (bind _asbp_projectile_grenade (cast `/Game/sA_Megapack_v1/sA_ShootingVfxPack/Blueprints/BP_Projectile_Grenade` OtherActor))
          (bind _asbp_grenadier_1 (cast `/Game/Blueprints/BP_Grenadier1` (`Actor.Instigator` _asbp_projectile_grenade)))
          (if (not (`self.IsMonster`))
            (`/Engine/EditorBlueprintResources/StandardMacros.DoOnce` false :!label _label_3
              (:`Completed`
                (bind _output_get_3 (set `self.HealthPoints` (- (`self.HealthPoints`) 42)))
                (if (<= _output_get_3 0)
                  (`self.PlayerDeath`)
                  (`KismetSystemLibrary.PrintString` (`KismetStringLibrary.Concat_StrStr` _returnvalue ": CHARACTER DIES"))
                  (else
                    (`GameplayStatics.SpawnEmitterAttached` "/Game/Realistic_Starter_VFX_Pack_Vol2/Particles/Blood/P_Blood_Splat_Cone.P_Blood_Splat_Cone" (`self.Mesh`) "None" (0.0 0.0 0.0) (struct) (2.0 2.0 2.0))
                    (`KismetSystemLibrary.PrintString` (`KismetStringLibrary.Concat_StrStr` _returnvalue ":" (`KismetStringLibrary.Conv_IntToString` _output_get_3)))))
                (`KismetSystemLibrary.Delay` (`/Game/Blueprints/BP_LifePoints/BP_LifePointsCharacter.DelayBetweenAttacks` _asbp_grenadier_1))
                (goto _label_3 :!via `Reset`)))))))))

(event `self.ReceiveBeginPlay`
  (bind _returnvalue (`|CreateWidget` "/Game/Blueprints/BP_LifePoints/WBP_HealthBar.WBP_HealthBar_C"))
  (bind _output_get (set `self.HealthBar` _returnvalue))
  (cast `/Game/Blueprints/BP_Player` self)
  (`UserWidget.AddToViewport` _output_get 0)
  (set `self.MaxHealth` (`self.HealthPoints`))
  (set `self.SpawnTransform` (`self.GetTransform`)))

(event `self.ReceiveTick`
  (params (DeltaSeconds :type "Float (single-precision)"))
  (`/Game/Blueprints/BP_LifePoints/WBP_HealthBar.Update Value` (`self.HealthBar`) (`self.HealthPoints`)))

(event `Refill Health`
  (set `self.HealthPoints` (`self.MaxHealth`)))

(fn `UserConstructionScript`)