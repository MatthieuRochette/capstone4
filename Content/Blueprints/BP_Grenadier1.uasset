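; BP_Grenadier1 is an enemy character that chases the player and throws grenade volleys, with template-style movement and look input bindings also present.
; Player overlap with its sphere clears Idle and starts a looping Throwing timer that moves it toward a standoff point near the player.
; Within range it stops, faces the player and spawns randomly scattered grenade projectiles.
; Events set state flags for throwing, damage aggro and delayed death.
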(event `InputAxis|MoveForward`
  (params (AxisValue :type "Float (single-precision)"))
  ;[1 1 1] Move action
  (`self.AddMovementInput` (`self.GetActorForwardVector`) AxisValue))

(event `InputAction|Jump`
  (params (Key :type "Key Structure"))
  ;[1 1 1] Jump action
  (:`Pressed`
    (`self.Jump`))
  (:`Released`
    (`self.StopJumping`)))

(event `InputAxis|MoveRight`
  (params (AxisValue :type "Float (single-precision)"))
  ;[1 1 1] Move action
  (`self.AddMovementInput` (`self.GetActorRightVector`) AxisValue))

(event `InputAxis|LookUp`
  (params (AxisValue :type "Float (single-precision)"))
  ;[1 1 1] LookUp
  (`self.AddControllerPitchInput` AxisValue))

(event `InputAxis|Turn`
  (params (AxisValue :type "Float (single-precision)"))
  ;[1 1 1] Turn action
  (`self.AddControllerYawInput` AxisValue))

(event `self.Sphere.OnComponentBeginOverlap`
  (params (OverlappedComponent :type "PrimitiveComponent Object Reference") (OtherActor :type "Actor Object Reference") (OtherComp :type "PrimitiveComponent Object Reference") (OtherBodyIndex :type Integer) (bFromSweep :type Boolean) (SweepResult :type "HitResult Structure (by ref)"))
  (if (== OtherActor (`GameplayStatics.GetPlayerCharacter` 0))
    (set `self.idle` false)
    (`KismetSystemLibrary.K2_SetTimerDelegate` (delegate `Throwing`) 0.5 (== (`self.idle`) false))))

(event `Throwing`
  (bind _returnvalue (`GameplayStatics.GetPlayerCharacter` 0))
  (bind _returnvalue_2 (`self.GetTransform`))
  (bind _returnvalue_3 (`self.K2_GetActorLocation` _returnvalue))
  (bind _returnvalue_4 (`KismetMathLibrary.FindLookAtRotation` (`self.K2_GetActorLocation`) (`self.K2_GetActorLocation` (`GameplayStatics.GetPlayerCharacter` 0))))
  (if (not (`self.idle`))
    (set `self.walk` true)
    (`AIBlueprintHelperLibrary.SimpleMoveToLocation` (`self.GetController`) (- _returnvalue_3 (* (`KismetMathLibrary.GetDirectionUnitVector` _returnvalue_3 (`self.K2_GetActorLocation`)) -500.0)))
    (if (<= (`self.GetDistanceTo` _returnvalue) 1000.0)
      (set `self.isThrowing` true)
      (`NavMovementComponent.StopActiveMovement` (`self.CharacterMovement`))
      (`SceneComponent.K2_SetWorldRotation` (`self.Mesh`) _returnvalue_4 false false)
      (for _ (range 5)
        (`|SpawnActorFromClass` "/Game/sA_Megapack_v1/sA_ShootingVfxPack/Blueprints/BP_Projectile_Grenade.BP_Projectile_Grenade_C" (`KismetMathLibrary.MakeTransform` (`KismetMathLibrary.MakeVector` (+ (.x (.location _returnvalue_2)) (`KismetMathLibrary.RandomFloatInRange` -100.0 100.0)) (+ (.y (.location _returnvalue_2)) (`KismetMathLibrary.RandomFloatInRange` -100.0 100.0)) (+ (.z (.location _returnvalue_2)) 200.0 (`KismetMathLibrary.RandomFloatInRange` 0.0 50.0))) _returnvalue_4 (.scale _returnvalue_2)) "Undefined" "OverrideRootScale" null self))
      (else
        (set `self.isThrowing` false)))))

(event `ThrowEnd`
  (set `self.isThrowing` false))

(event `self.Die`
  (`NavMovementComponent.StopActiveMovement` (`self.CharacterMovement`))
  (set `self.death` true)
  (`KismetSystemLibrary.Delay` 0.66666)
  (`self.K2_DestroyActor`))

(event `self.TakeDmgs`
  (set `self.idle` false))

(fn `UserConstructionScript`)