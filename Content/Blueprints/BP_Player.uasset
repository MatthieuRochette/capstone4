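; Player character with movement, look, jump, a first/third-person toggle and rifle fire.
; The toggle swaps mesh, arms and weapon visibility while a timeline extends or retracts the camera boom.
; Fire is rate-limited by a resetting DoOnce and casts player 0 to BP_Player_Interact for FireShot.
; FireShot debug-traces from the active weapon's muzzle along camera forward, then spawns a BP_AssaultRifleRound toward that target with a pitch offset.
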(event `InputAxis|MoveForward`
  (params (AxisValue :type "Float (single-precision)"))
  ;[1 1 1] Move action
  (`self.AddMovementInput` (`self.GetActorForwardVector`) AxisValue))

(event `InputAction|Jump`
  (params (Key :type "Key Structure"))
  ;[1 1 1] Jump action
  (:`Pressed`
    (`self.Jump`))
  (:`Released`
    (`self.StopJumping`)))

(event `InputAxis|MoveRight`
  (params (AxisValue :type "Float (single-precision)"))
  ;[1 1 1] Move action
  (`self.AddMovementInput` (`self.GetActorRightVector`) AxisValue))

(event `InputAxis|LookUp`
  (params (AxisValue :type "Float (single-precision)"))
  ;[1 1 1] LookUp
  (`self.AddControllerPitchInput` AxisValue))

(event `InputAxis|Turn`
  (params (AxisValue :type "Float (single-precision)"))
  ;[1 1 1] Turn action
  (`self.AddControllerYawInput` AxisValue))

(event `InputAction|Toggle Third Person`
  (params (Key :type "Key Structure"))
  ;[1 1 1] FPS to TPS and back
  (:`Pressed`
    (`/Engine/EditorBlueprintResources/StandardMacros.FlipFlop`
      (:`A`
        (set `self.IsTPS` true)
        (`PrimitiveComponent.SetOwnerNoSee` (`self.Mesh`) false)
        (`PrimitiveComponent.SetOnlyOwnerSee` (`self.Mesh`) true)
        (`SceneComponent.SetVisibility` (`self.SK_Weapon_TPS`) true true)
        (`SceneComponent.SetVisibility` (`self.Arms`) false true)
        (bind (_direction _target_arm_lenght) (`Timeline|Third person view timeline` :!label _label)
          (:`Update`
            (set `SpringArmComponent.TargetArmLength` _target_arm_lenght (`self.camera boom`)))
          (:`Finished`
            (if (`|EnumEquality` _direction "Backward")
              (`PrimitiveComponent.SetOwnerNoSee` (`self.Mesh`) true)
              (`SceneComponent.SetVisibility` (`self.Arms`) true true)
              (`SceneComponent.SetVisibility` (`self.SK_Weapon_TPS`) false true)))))
      (:`B`
        (set `self.IsTPS` false)
        (goto _label :!via `Reverse`)))))

(event `InputAction|Fire`
  (params (Key :type "Key Structure"))
  (:`Pressed`
    (`/Engine/EditorBlueprintResources/StandardMacros.DoOnce` false :!label _label_2
      (:`Completed`
        (bind _asbp_player_interact (cast `/Game/Worksite_League/InteractableActor/BP_Player_Interact` (`GameplayStatics.GetPlayerCharacter` 0)))
        (if (`self.IsTPS`)
          (`SkeletalMeshComponent.PlayAnimation` (`self.SK_Weapon_TPS`) "/Game/MilitaryWeapSilver/Weapons/Animations/Fire_Rifle_W.Fire_Rifle_W" false)
          (else
            (set `self.Shooting` true)
            (`SkeletalMeshComponent.PlayAnimation` (`self.SK_Weapon_FPS`) "/Game/MilitaryWeapSilver/Weapons/Animations/Fire_Rifle_W.Fire_Rifle_W" false)))
        (`self.FireShot` _asbp_player_interact)
        (`KismetSystemLibrary.Delay` 0.1)
        (set `self.Shooting` false)
        (`KismetSystemLibrary.Delay` 0.1)
        (goto _label_2 :!via `Reset`)))))

(fn `FireShot`
  (params (InteractPlayer :type "/Game/Worksite_League/InteractableActor/BP_Player_Interact Object Reference"))
  (bind _returnvalue (`SceneComponent.GetSocketLocation` (`/Game/Blueprints/BP_Player.SK_Weapon_FPS` InteractPlayer) "RoundSpawn"))
  (bind _returnvalue_2 (`SceneComponent.GetSocketLocation` (`/Game/Blueprints/BP_Player.SK_Weapon_TPS` InteractPlayer) "RoundSpawn"))
  (bind _returnvalue_3 (+ _returnvalue (* (`KismetMathLibrary.GetForwardVector` (`SceneComponent.K2_GetComponentRotation` (`/Game/Blueprints/BP_Player.Camera` InteractPlayer))) 5000)))
  (bind _returnvalue_4 (+ _returnvalue_2 (* (`KismetMathLibrary.GetForwardVector` (`SceneComponent.K2_GetComponentRotation` (`/Game/Blueprints/BP_Player.Camera` InteractPlayer))) 5000)))
  (`|ExecutionSequence`
    (:`then_0`
      (if (`self.IsTPS`)
        (bind (_outhit _returnvalue_5) (`KismetSystemLibrary.LineTraceSingle` :`Start` _returnvalue_2 :`End` _returnvalue_4 :`TraceChannel` "TraceTypeQuery1" :`DrawDebugType` "ForDuration"))
        (else
          (bind (_outhit_2 _returnvalue_6) (`KismetSystemLibrary.LineTraceSingle` :`Start` _returnvalue :`End` _returnvalue_3 :`TraceChannel` "TraceTypeQuery1" :`DrawDebugType` "ForDuration")))))
    (:`then_1`
      (if (`self.IsTPS`)
        (if _returnvalue_5
          (bind _outhit_3 (`KismetSystemLibrary.LineTraceSingle` :`Start` _returnvalue_2 :`End` (+ (`.Location` (`GameplayStatics.BreakHitResult` _outhit)) (* (`.ImpactNormal` (`GameplayStatics.BreakHitResult` _outhit)) -1)) :`TraceChannel` "TraceTypeQuery1" :`DrawDebugType` "ForDuration"))
          (bind (_returnvalue_roll _returnvalue_pitch _returnvalue_yaw) (`KismetMathLibrary.BreakRotator` (`KismetMathLibrary.FindLookAtRotation` _returnvalue_2 (`.TraceEnd` (`GameplayStatics.BreakHitResult` _outhit_3)))))
          (`|SpawnActorFromClass` "/Game/MilitaryWeapSilver/Rounds/BP_AssaultRifleRound.BP_AssaultRifleRound_C" (`KismetMathLibrary.MakeTransform` _returnvalue_2 (`KismetMathLibrary.MakeRotator` _returnvalue_roll (- _returnvalue_pitch 3.0) _returnvalue_yaw) (0.1 0.1 0.1)) "AlwaysSpawn" "OverrideRootScale" null self)
          (else
            (bind _outhit_4 (`KismetSystemLibrary.LineTraceSingle` :`Start` _returnvalue_2 :`End` _returnvalue_4 :`TraceChannel` "TraceTypeQuery1" :`DrawDebugType` "ForDuration"))
            (bind (_returnvalue_roll_2 _returnvalue_pitch_2 _returnvalue_yaw_2) (`KismetMathLibrary.BreakRotator` (`KismetMathLibrary.FindLookAtRotation` _returnvalue_2 (`.TraceEnd` (`GameplayStatics.BreakHitResult` _outhit_4)))))
            (`|SpawnActorFromClass` "/Game/MilitaryWeapSilver/Rounds/BP_AssaultRifleRound.BP_AssaultRifleRound_C" (`KismetMathLibrary.MakeTransform` _returnvalue_2 (`KismetMathLibrary.MakeRotator` _returnvalue_roll_2 (- _returnvalue_pitch_2 3.0) _returnvalue_yaw_2) (0.1 0.1 0.1)) "AlwaysSpawn" "OverrideRootScale" null self)))))
    (:`then_2`
      (if (`self.IsTPS`)
        _
        (elif _returnvalue_6
          (bind _outhit_5 (`KismetSystemLibrary.LineTraceSingle` :`Start` _returnvalue :`End` (+ (`.Location` (`GameplayStatics.BreakHitResult` _outhit_2)) (* (`.ImpactNormal` (`GameplayStatics.BreakHitResult` _outhit_2)) -1)) :`TraceChannel` "TraceTypeQuery1" :`DrawDebugType` "ForDuration"))
          (bind (_returnvalue_roll_3 _returnvalue_pitch_3 _returnvalue_yaw_3) (`KismetMathLibrary.BreakRotator` (`KismetMathLibrary.FindLookAtRotation` _returnvalue (`.TraceEnd` (`GameplayStatics.BreakHitResult` _outhit_5)))))
          (`|SpawnActorFromClass` "/Game/MilitaryWeapSilver/Rounds/BP_AssaultRifleRound.BP_AssaultRifleRound_C" (`KismetMathLibrary.MakeTransform` _returnvalue (`KismetMathLibrary.MakeRotator` _returnvalue_roll_3 (- _returnvalue_pitch_3 3.0) _returnvalue_yaw_3) (0.1 0.1 0.1)) "AlwaysSpawn" "OverrideRootScale" null self)
          (else
            (bind _outhit_6 (`KismetSystemLibrary.LineTraceSingle` :`Start` _returnvalue :`End` _returnvalue_3 :`TraceChannel` "TraceTypeQuery1" :`DrawDebugType` "ForDuration"))
            (bind (_returnvalue_roll_4 _returnvalue_pitch_4 _returnvalue_yaw_4) (`KismetMathLibrary.BreakRotator` (`KismetMathLibrary.FindLookAtRotation` _returnvalue (`.TraceEnd` (`GameplayStatics.BreakHitResult` _outhit_6)))))
            (`|SpawnActorFromClass` "/Game/MilitaryWeapSilver/Rounds/BP_AssaultRifleRound.BP_AssaultRifleRound_C" (`KismetMathLibrary.MakeTransform` _returnvalue (`KismetMathLibrary.MakeRotator` _returnvalue_roll_4 (- _returnvalue_pitch_4 3.0) _returnvalue_yaw_4) (0.1 0.1 0.1)) "AlwaysSpawn" "OverrideRootScale" null self)))))))

(fn `UserConstructionScript`
  (`SceneComponent.K2_AttachToComponent` (`self.SK_Weapon_FPS`) (`self.Arms`) "GripPoint" "KeepRelative" "KeepRelative" "KeepRelative" true)
  (`SceneComponent.K2_AttachToComponent` (`self.SK_Weapon_TPS`) (`self.Mesh`) "hand_r_weapon" "KeepRelative" "KeepRelative" "KeepRelative" true))