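; BP_Sploder is an exploding enemy character that chases the player once it perceives them or takes damage.
; While alive and aggroed, it issues AIMoveTo on the player every Tick and drives attack and death flags on BP_Chaser_Anim.
; Capsule contact with the player or Die spawns explosion effects and sound, then both share a death tail that calls parent Die after a delay.
; No explosion damage is applied in this graph.
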(event `self.ReceiveTick`
  (params (DeltaSeconds :type "Float (single-precision)"))
  (if (`self.Attack`)
    (if (`self.IsAlive`)
      (`|AIMoveTo` self (0.0 0.0 0.0) (`GameplayStatics.GetPlayerCharacter` 0)))))

(event `self.AIPerception.OnTargetPerceptionUpdated`
  (params (Actor :type "Actor Object Reference") (Stimulus :type "AIStimulus Structure"))
  (cast `/Game/Blueprints/BP_Player` Actor)
  (set `self.Attack` true)
  (bind _asbp_chaser_anim (cast `/Game/CityofBrass_Enemies/Meshes/Enemy/Corpse/BP_Chaser_Anim` (`SkeletalMeshComponent.GetAnimInstance` (`self.Mesh`))))
  (set `/Game/CityofBrass_Enemies/Meshes/Enemy/Corpse/BP_Chaser_Anim.attack` true _asbp_chaser_anim))

(event `self.CapsuleComponent.OnComponentHit`
  (params (HitComponent :type "PrimitiveComponent Object Reference") (OtherActor :type "Actor Object Reference") (OtherComp :type "PrimitiveComponent Object Reference") (NormalImpulse :type "Vector Structure") (Hit :type "HitResult Structure (by ref)"))
  (bind _returnvalue (`SceneComponent.K2_GetComponentLocation` (`self.CapsuleComponent`)))
  (if (`self.IsAlive`)
    (cast `/Game/Blueprints/BP_Player` OtherActor)
    (`/Engine/EditorBlueprintResources/StandardMacros.DoOnce` false
      (:`Completed`
        (`GameplayStatics.SpawnEmitterAtLocation` "/Game/StarterContent/Particles/P_Explosion.P_Explosion" _returnvalue)
        (`GameplayStatics.SpawnSoundAtLocation` "/Game/StarterContent/Audio/Explosion_Cue.Explosion_Cue" _returnvalue (struct) 1.0 1.0 0.0 null null)
        (`KismetSystemLibrary.Delay` 0.1)
        (set `self.IsAlive` false :!label _label)
        (bind _asbp_chaser_anim (cast `/Game/CityofBrass_Enemies/Meshes/Enemy/Corpse/BP_Chaser_Anim` (`SkeletalMeshComponent.GetAnimInstance` (`self.Mesh`))))
        (set `/Game/CityofBrass_Enemies/Meshes/Enemy/Corpse/BP_Chaser_Anim.death` true _asbp_chaser_anim)
        (`KismetSystemLibrary.Delay` 2.8333)
        (`parent.Die`)))))

(event `self.Die`
  (bind _returnvalue (`SceneComponent.K2_GetComponentLocation` (`self.CapsuleComponent`)))
  (`NavMovementComponent.StopActiveMovement` (`self.CharacterMovement`))
  (`GameplayStatics.SpawnEmitterAtLocation` "/Game/StarterContent/Particles/P_Explosion.P_Explosion" _returnvalue)
  (`GameplayStatics.SpawnSoundAtLocation` "/Game/StarterContent/Audio/Explosion_Cue.Explosion_Cue" _returnvalue (struct) 1.0 1.0 0.0 null null)
  (goto _label))

(event `self.TakeDamages`
  (bind _asbp_chaser_anim (cast `/Game/CityofBrass_Enemies/Meshes/Enemy/Corpse/BP_Chaser_Anim` (`SkeletalMeshComponent.GetAnimInstance` (`self.Mesh`))))
  (set `/Game/CityofBrass_Enemies/Meshes/Enemy/Corpse/BP_Chaser_Anim.attack` true _asbp_chaser_anim)
  (set `self.Attack` true))

(fn `UserConstructionScript`)