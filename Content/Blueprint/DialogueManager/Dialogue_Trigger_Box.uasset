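; Trigger box actor that shows a dialogue widget on screen when the player character overlaps it.
; On overlap it creates a Dialogue_Widget, adds it to the viewport with its configured text, then removes it after a set duration.
; An IsUsed flag blocks retriggering while the dialogue is showing.
; An OnlyOnce option destroys the actor after the first display.
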(event `self.RemoveDialogueBox`
  ;[1 0.02313 0.8304] Dialogue Manager Class
  (`self.EndDialogue` self)
  (`self.K2_DestroyActor` self))

(event `self.EndDialogue`
  ;[1 0.02313 0.8304] Dialogue Manager Class
  (`Widget.RemoveFromParent` (`self.DialogueWidget`))
  (set `self.IsUsed` false))

(event `self.TriggerDialogue`
  ;[1 0.02313 0.8304] Dialogue Manager Class
  (if (not (`self.IsUsed`))
    (bind _returnvalue (`|CreateWidget` "/Game/Blueprint/DialogueManager/Dialogue_Widget.Dialogue_Widget_C" (`GameplayStatics.GetPlayerController` 0)))
    (`|ExecutionSequence`
      (:`then_0`
        (bind _output_get (set `self.DialogueWidget` _returnvalue))
        (`UserWidget.AddToViewport` _output_get 0)
        (set `/Game/Blueprint/DialogueManager/Dialogue_Widget.DialogueText` (`self.TextToDisplay`) _output_get)
        (`KismetSystemLibrary.Delay` (`self.Duration`))
        (`self.EndDialogue` self)
        (if (`self.OnlyOnce`)
          (`self.RemoveDialogueBox` self)))
      (:`then_1`
        (set `self.IsUsed` true)))))

(event `self.Box.OnComponentBeginOverlap`
  (params (OverlappedComponent :type "PrimitiveComponent Object Reference") (OtherActor :type "Actor Object Reference") (OtherComp :type "PrimitiveComponent Object Reference") (OtherBodyIndex :type Integer) (bFromSweep :type Boolean) (SweepResult :type "HitResult Structure (by ref)"))
  ;[0.8587 0.2311 1] Dialogue Box Overlap
  (if (== OtherActor (`GameplayStatics.GetPlayerCharacter` 0))
    (`self.TriggerDialogue`)))

(fn `UserConstructionScript`)